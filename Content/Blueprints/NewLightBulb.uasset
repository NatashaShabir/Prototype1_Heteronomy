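; Light bulb Blueprint that switches between lit and dull states by swapping the mesh material and showing or hiding its point light.
; On BeginPlay, StatusCheck applies the initial on/off state, then optionally starts flickering and changes colour.
; Flicker runs a looping timer that randomly calls Toggle and clears itself after a toggle once IsFlickering is false.
; ChangeColour applies a new light colour and green bulb material only when IsGreen is set.
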(event `self.ReceiveBeginPlay`
  ;[1 1 1] Begin Play
  (`self.StatusCheck`))

(event `Flicker`
  ;[1 1 1] Flicker
  (bind _returnvalue (`KismetSystemLibrary.K2_SetTimerDelegate` (delegate `FlickerEvent`) 0.1 true)))

(event `FlickerEvent`
  ;[1 1 1] Flicker
  (if (> (`KismetMathLibrary.RandomIntegerInRange` 1 5) 3)
    (`self.Toggle`)
    (if (not (`self.IsFlickering`))
      (`KismetSystemLibrary.K2_ClearAndInvalidateTimerHandle` (stale `Flicker` _returnvalue)))))

(event `On`
  ;[1 1 1] On/Off
  (`PrimitiveComponent.SetMaterial` (`self.StaticMesh`) 0 "/Game/Materials/BrightBulb.BrightBulb")
  (`SceneComponent.SetVisibility` (`self.PointLight`) true false)
  (set `self.IsOn` true))

(event `Off`
  ;[1 1 1] On/Off
  (`PrimitiveComponent.SetMaterial` (`self.StaticMesh`) 0 "/Game/Materials/DullBulb.DullBulb")
  (`SceneComponent.SetVisibility` (`self.PointLight`) false false)
  (set `self.IsOn` false))

(event `Toggle`
  ;[1 1 1] Toggle
  (if (`self.IsOn`)
    (set `self.IsOn` false)
    (`self.Off`)
    (else
      (set `self.IsOn` true)
      (`self.On`))))

(event `ChangeColour`
  (if (`self.IsGreen`)
    (`LightComponent.SetLightColor` (`self.PointLight`) (`self.NewColour`) true)
    (`PrimitiveComponent.SetMaterial` (`self.StaticMesh`) 0 "/Game/Materials/GreenBulb.GreenBulb")))

(fn `StatusCheck`
  (if (`self.IsOn`)
    (`self.On`)
    (else
      (`self.Off`)))
  (if (`self.IsFlickering`)
    (`self.Flicker`))
  (if (`self.DifferentColour`)
    (`self.ChangeColour`)))

(fn `UserConstructionScript`)