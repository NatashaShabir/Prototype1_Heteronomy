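; Dialogue trigger volume that freezes the first-person player on first overlap and plays a conversation in a DialogueWidget.
; BeginPlay collects DialogueLines data table rows matching its ConversationID.
; The overlap, and each later TriggerDialogue event, increments the line counter and displays the text GetDialogueLine finds for that LineID.
; Without exactly one matching line, GetDialogueLine ends the conversation, resetting the counter, removing the widget and restoring movement.
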(event `self.ReceiveBeginPlay`
  ;[1 1 1] Sets which dialogue lines to use for this dialogue trigger
  (bind _outrownames (`DataTableFunctionLibrary.GetDataTableRowNames` "/Game/Blueprints/Dialogue/DialogueLines_-_Sheet1.DialogueLines_-_Sheet1"))
  (for _array_element _outrownames
    (bind _returnvalue (`|GetDataTableRow` "/Game/Blueprints/Dialogue/DialogueLines_-_Sheet1.DialogueLines_-_Sheet1" _array_element)
      (:`then`
        (if (== (`.Conversation_ID_3_1D5FDF274DDD67B5169C75B86B61D172` (break `/Game/Blueprints/Dialogue/DialogueStructure` _returnvalue)) (`self.Conversation_ID`))
          (`KismetArrayLibrary.Array_Add` (`self.MyDialogue`) _array_element))))))

(event `self.Box.OnComponentBeginOverlap`
  (params (OverlappedComponent :type "PrimitiveComponent Object Reference") (OtherActor :type "Actor Object Reference") (OtherComp :type "PrimitiveComponent Object Reference") (OtherBodyIndex :type Integer) (bFromSweep :type Boolean) (SweepResult :type "HitResult Structure (by ref)"))
  (`/Engine/EditorBlueprintResources/StandardMacros.DoOnce` false
    (:`Completed`
      (bind _asfirst_person_character (cast `/Game/FirstPersonBP/Blueprints/FirstPersonCharacter` OtherActor))
      (set `self.Player` _asfirst_person_character)
      (`ActorComponent.SetActive` (`Character.CharacterMovement` (`self.Player`)) false false)
      (set `self.IsPlayer` true)
      (`/Engine/EditorBlueprintResources/StandardMacros.IncrementInt` (`self.LineCurrent`)
        (:`  `
          (`/Engine/EditorBlueprintResources/StandardMacros.IsValid` (`self.DialogueWidget`) :!label _label
            (:`Is Valid`
              (bind _returnedline (`self.GetDialogueLine`))
              (set `/Game/UI/DialogueWidget.DialogueText` _returnedline (`self.DialogueWidget`)))
            (:`Is Not Valid`
              (bind _returnvalue (`|CreateWidget` "/Game/UI/DialogueWidget.DialogueWidget_C"))
              (bind _output_get (set `self.DialogueWidget` _returnvalue))
              (`UserWidget.AddToViewport` _output_get 0)
              (bind _returnedline_2 (`self.GetDialogueLine`))
              (set `/Game/UI/DialogueWidget.DialogueText` _returnedline_2 (`self.DialogueWidget`)))))))))

(event `/Game/Blueprints/InteractInterface.TriggerDialogue`
  (`/Engine/EditorBlueprintResources/StandardMacros.IncrementInt` (`self.LineCurrent`)
    (:`  `
      (goto _label))))

(fn `GetDialogueLine`
  (returns (returnedLine :type Text))
  (locals (ReturnedLines :type "Array of Text"))
  (for _array_element (`self.MyDialogue`)
    (bind _returnvalue (`|GetDataTableRow` "/Game/Blueprints/Dialogue/DialogueLines_-_Sheet1.DialogueLines_-_Sheet1" _array_element)
      (:`then`
        (bind (_conversation_id _line_id _dialogue) (break `/Game/Blueprints/Dialogue/DialogueStructure` _returnvalue))
        (if (and (== _conversation_id (`self.Conversation_ID`)) (== _line_id (`self.LineCurrent`)))
          (`KismetArrayLibrary.Array_Add` (`local.ReturnedLines`) _dialogue)))))
  (if (== (`KismetArrayLibrary.Array_Length` (`local.ReturnedLines`)) 1)
    (return (`|GetArrayItem` (`local.ReturnedLines`)))
    (else
      (set `self.IsPlayer` false)
      (set `self.LineCurrent` 0)
      (`Widget.RemoveFromParent` (`self.DialogueWidget`))
      (`ActorComponent.SetActive` (`Character.CharacterMovement` (`self.Player`)) true false))))

(fn `UserConstructionScript`)