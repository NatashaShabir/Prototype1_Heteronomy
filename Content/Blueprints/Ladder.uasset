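; Ladder actor that lets the first-person character climb while inside its Box trigger volume.
; On overlap it flags the character as IsOnLadder, stops its movement, switches to Flying mode and disables capsule gravity.
; Leaving the box clears the flag and restores Walking mode and gravity.
; Climbing input is not handled here, only the movement state.
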(event `self.Box.OnComponentBeginOverlap`
  (params (OverlappedComponent :type "PrimitiveComponent Object Reference") (OtherActor :type "Actor Object Reference") (OtherComp :type "PrimitiveComponent Object Reference") (OtherBodyIndex :type Integer) (bFromSweep :type Boolean) (SweepResult :type "HitResult Structure (by ref)"))
  (bind _asfirst_person_character (cast `/Game/FirstPersonBP/Blueprints/FirstPersonCharacter` OtherActor))
  (set `/Game/FirstPersonBP/Blueprints/FirstPersonCharacter.IsOnLadder` true _asfirst_person_character)
  (bind _charactermovement (`Character.CharacterMovement` _asfirst_person_character))
  (`MovementComponent.StopMovementImmediately` _charactermovement)
  (`CharacterMovementComponent.SetMovementMode` _charactermovement "MOVE_Flying" 0)
  (`PrimitiveComponent.SetEnableGravity` (`Character.CapsuleComponent` _asfirst_person_character) false))

(event `self.Box.OnComponentEndOverlap`
  (params (OverlappedComponent :type "PrimitiveComponent Object Reference") (OtherActor :type "Actor Object Reference") (OtherComp :type "PrimitiveComponent Object Reference") (OtherBodyIndex :type Integer))
  (bind _asfirst_person_character (cast `/Game/FirstPersonBP/Blueprints/FirstPersonCharacter` OtherActor))
  (set `/Game/FirstPersonBP/Blueprints/FirstPersonCharacter.IsOnLadder` false _asfirst_person_character)
  (`CharacterMovementComponent.SetMovementMode` (`Character.CharacterMovement` _asfirst_person_character) "MOVE_Walking" 0)
  (`PrimitiveComponent.SetEnableGravity` (`Character.CapsuleComponent` _asfirst_person_character) true))

(fn `UserConstructionScript`)